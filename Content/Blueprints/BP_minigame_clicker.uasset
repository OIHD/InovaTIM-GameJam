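; Clicker minigame actor that opens the W_minigame_clicker widget with UI-only input when its box is overlapped, and cancels it when the overlap ends.
; Setter functions flag three "Civi" targets; Tick polls them, while also counting down TimeRepeat, which triggers nothing.
; Once all three are set, Win closes the widget, restores game input, adds PrizeResource to the player's inventory and destroys the actor.
; The Tekrarla repeat function is an empty stub.
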(event OnComponentBeginOverlap(Box)
  (params (OverlappedComponent :type Primitive%20Component%20Object%20Reference) (OtherActor :type Actor%20Object%20Reference) (OtherComp :type Primitive%20Component%20Object%20Reference) (OtherBodyIndex :type Integer) (bFromSweep :type Boolean) (SweepResult :type Hit%20Result%20Structure%20%28by%20ref%29))
  (Development|PrintString "Minigame_1_started")
  (bind _returnvalue (UserInterface|CreateWidget "/Game/Blueprints/W_minigame_clicker.W_minigame_clicker_C"))
  (UserInterface|Viewport|AddtoViewport _returnvalue 0)
  (Input|SetInputModeUIOnly (Game|GetPlayerController 0) _returnvalue "DoNotLock"))

(event OnComponentEndOverlap(Box)
  (params (OverlappedComponent :type Primitive%20Component%20Object%20Reference) (OtherActor :type Actor%20Object%20Reference) (OtherComp :type Primitive%20Component%20Object%20Reference) (OtherBodyIndex :type Integer))
  (Widget|SetIsEnabled (stale OnComponentBeginOverlap(Box) _returnvalue) false)
  (Widget|RemovefromParent (stale OnComponentBeginOverlap(Box) _returnvalue))
  (Input|SetInputModeGameandUI (Game|GetPlayerController 0) 0 "DoNotLock" true)
  (Input|EnableInput 0)
  (Development|PrintString "minigame_1_cancelled"))

(event Custom|Timer
  (Variables|Default|SetTimeRepeat (Math|Float|Clamp(Float) (- (Variables|Default|GetTimeRepeat) (Utilities|Time|GetWorldDeltaSeconds)) 0.0 (Variables|Default|GetTimeRepeat)))
  (if (and (and (Variables|Default|Getcivi1) (Variables|Default|Getcivi2)) (Variables|Default|Getcivi3))
    (CallFunction|Win)))

(event Custom|win
  (bind _returnvalue (Game|GetPlayerController 0))
  (Variables|Default|Setcivi1 false)
  (Variables|Default|Setcivi2 false)
  (Variables|Default|Setcivi3 false)
  (Utilities|IsValid (stale OnComponentBeginOverlap(Box) _returnvalue)
    (:Is%20Valid
      (Widget|RemovefromParent (stale OnComponentBeginOverlap(Box) _returnvalue))
      (Input|SetInputModeGameOnly _returnvalue)
      (Input|EnableInput _returnvalue)
      (Development|PrintString "burada ui a return donecek")
      (Default|IncreaseResource (Variables|/Game/TopDown/Blueprints/BP_TopDownCharacter.BP_TopDownCharacter_C|GetInventoryComponent (Variables|Default|GetAs%20BP%20Top%20Down%20Character)) (Variables|Default|GetPrizeResource))
      (Utilities|IsValid _returnvalue
        (:Is%20Valid
          (Actor|DestroyActor)
          (CallFunction|Tekrarla))))))

(event EventBeginPlay
  (Variables|Default|Setcivi1 false)
  (Variables|Default|Setcivi2 false)
  (Variables|Default|Setcivi3 false)
  (bind _asbp_top_down_character (Utilities|Casting|CastToBP_TopDownCharacter (Game|GetPlayerCharacter 0)))
  (Variables|Default|SetAs%20BP%20Top%20Down%20Character _asbp_top_down_character))

(event Collision|EventActorBeginOverlap
  (params (OtherActor :type Actor%20Object%20Reference)))

(event EventTick
  (params (DeltaSeconds :type Float%20%28single-precision%29))
  (CallFunction|Timer))

(fn ConstructionScript)

(fn FCivi1
  (Variables|Default|Setcivi1 true))

(fn FCivi2
  (Variables|Default|Setcivi2 true))

(fn FCivi3
  (Variables|Default|Setcivi3 true))

(fn Tekrarla
  (return))