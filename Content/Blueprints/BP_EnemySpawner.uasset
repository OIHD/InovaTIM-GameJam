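; Enemy spawner actor that creates BP_EnemyAi enemies at its own transform, gated by the day state on the player's StateComponent.
; BeginPlay caches the player as BP_TopDownCharacter and queries BP_Shield actors without using the result.
; Tick sets CanSpawn while DayState matches its target value and calls Spawn, which creates EnemyCount enemies.
; Spawning repeats every frame during that state, as nothing limits it to once.
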(event EventBeginPlay
  (bind _asbp_top_down_character (Utilities|Casting|CastToBP_TopDownCharacter (Game|Player|GetPlayerPawn 0)))
  (Variables|Default|SetAs%20BP%20Top%20Down%20Character _asbp_top_down_character)
  (Actor|GetAllActorsOfClass "/Game/Blueprints/BP_Shield.BP_Shield_C"))

(event Collision|EventActorBeginOverlap
  (params (OtherActor :type Actor%20Object%20Reference)))

(event EventTick
  (params (DeltaSeconds :type Float%20%28single-precision%29))
  (if (Utilities|Enum|Equal(Enum) (Variables|/Game/Blueprints/Components/StateComponent.StateComponent_C|GetDayState (Variables|/Game/TopDown/Blueprints/BP_TopDownCharacter.BP_TopDownCharacter_C|GetStateComponent (Variables|Default|GetAs%20BP%20Top%20Down%20Character))) "NewEnumerator1")
    (Variables|Default|SetCanSpawn true)
    (CallFunction|Spawn)
    (else
      (Variables|Default|SetCanSpawn false))))

(fn ConstructionScript)

(fn Spawn
  (if (Variables|Default|GetCanSpawn)
    (for _index (range 0 (- (Variables|Default|GetEnemyCount) 1))
      (Game|SpawnActorfromClass "/Game/EnemyAi/BP_EnemyAi.BP_EnemyAi_C" (Transformation|GetActorTransform) "Undefined" 0 0))))