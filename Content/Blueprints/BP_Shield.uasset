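; BP_Shield is a shield actor that loses health while BP_EnemyAi actors overlap its Sphere, and it adds a WBP_Health widget to the viewport on BeginPlay.
; Each enemy entry increments EnemyCount, which never decrements, and starts a looping one-second TakeDamage timer.
; While CanDamage is set, the timer subtracts Damage scaled by EnemyCount and prints "GameOver" regardless of remaining health.
; Any enemy leaving clears CanDamage.
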(event OnComponentBeginOverlap(Sphere)
  (params (OverlappedComponent :type Primitive%20Component%20Object%20Reference) (OtherActor :type Actor%20Object%20Reference) (OtherComp :type Primitive%20Component%20Object%20Reference) (OtherBodyIndex :type Integer) (bFromSweep :type Boolean) (SweepResult :type Hit%20Result%20Structure%20%28by%20ref%29))
  (Utilities|Casting|CastToBP_EnemyAi OtherActor)
  (Math|Integer|IncrementInt (Variables|Default|GetEnemyCount)
    (:%20%20
      (Variables|Default|SetCanDamage true)
      (Utilities|Time|SetTimerbyEvent (delegate Custom|TakeDamage) 1.0 true))))

(event OnComponentEndOverlap(Sphere)
  (params (OverlappedComponent :type Primitive%20Component%20Object%20Reference) (OtherActor :type Actor%20Object%20Reference) (OtherComp :type Primitive%20Component%20Object%20Reference) (OtherBodyIndex :type Integer))
  (Utilities|Casting|CastToBP_EnemyAi OtherActor)
  (Variables|Default|SetCanDamage false))

(event Custom|TakeDamage
  (if (Variables|Default|GetCanDamage)
    (bind _output_get (Variables|Default|SetCurrentHealth (- (Variables|Default|GetCurrentHealth) (* (Variables|Default|GetDamage) (Variables|Default|GetEnemyCount)))))
    (if (<= _output_get 0.0)
      _
      (else
        _))
    (Development|PrintString "GameOver")))

(event EventBeginPlay
  (bind _returnvalue (UserInterface|CreateWidget "/Game/Blueprints/WidgetBlueprints/WBP_Health.WBP_Health_C"))
  (UserInterface|Viewport|AddtoViewport _returnvalue 0))

(event Collision|EventActorBeginOverlap
  (params (OtherActor :type Actor%20Object%20Reference)))

(event EventTick
  (params (DeltaSeconds :type Float%20%28single-precision%29)))

(fn ConstructionScript)