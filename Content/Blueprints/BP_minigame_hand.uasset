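; BP_minigame_hand is a world trigger that starts a hand minigame and awards a resource on winning.
; Entering its box freezes the top-down character, plays an interact montage, then opens the W_minigame_hand widget in UI-only input.
; Tick polls Wingame, then closes the widget, grants PrizeResource, destroys the actor and restores movement.
; Leaving the box cancels the widget; six setter functions raise flags that are never read here.
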(event OnComponentBeginOverlap(Box)
  (params (OverlappedComponent :type Primitive%20Component%20Object%20Reference) (OtherActor :type Actor%20Object%20Reference) (OtherComp :type Primitive%20Component%20Object%20Reference) (OtherBodyIndex :type Integer) (bFromSweep :type Boolean) (SweepResult :type Hit%20Result%20Structure%20%28by%20ref%29))
  (bind _as_bp_top_down_character (Variables|Default|GetAs%20BP%20Top%20Down%20Character))
  (bind _charactermovement (Variables|/Script/Engine.Character|GetCharacterMovement _as_bp_top_down_character))
  (Variables|/Script/Engine.CharacterMovementComponent|SetMaxWalkSpeed _charactermovement 0.0)
  (Variables|/Script/Engine.CharacterMovementComponent|SetRotationRate _charactermovement "0, 0, 0")
  (Animation|Montage|PlayMontage (Variables|/Script/Engine.Character|GetMesh _as_bp_top_down_character) "/Game/Models/Character_Main/mc-robot_Anim_Interact_Montage.mc-robot_Anim_Interact_Montage"
    (:then
      (Utilities|FlowControl|Delay 0.5)
      (bind _returnvalue (UserInterface|CreateWidget "/Game/Blueprints/W_minigame_hand.W_minigame_hand_C"))
      (UserInterface|Viewport|AddtoViewport _returnvalue 0)
      (Input|SetInputModeUIOnly (Game|GetPlayerController 0) _returnvalue "DoNotLock"))))

(event OnComponentEndOverlap(Box)
  (params (OverlappedComponent :type Primitive%20Component%20Object%20Reference) (OtherActor :type Actor%20Object%20Reference) (OtherComp :type Primitive%20Component%20Object%20Reference) (OtherBodyIndex :type Integer))
  (Widget|SetIsEnabled (stale OnComponentBeginOverlap(Box) _returnvalue) false)
  (Widget|RemovefromParent (stale OnComponentBeginOverlap(Box) _returnvalue))
  (Input|SetInputModeGameandUI (Game|GetPlayerController 0) 0 "DoNotLock" false)
  (Input|EnableInput 0)
  (Development|PrintString "minigame_3_cancelled"))

(event Custom|Timer
  (bind _as_bp_top_down_character (Variables|Default|GetAs%20BP%20Top%20Down%20Character))
  (bind _charactermovement (Variables|/Script/Engine.Character|GetCharacterMovement _as_bp_top_down_character))
  (Variables|Default|SetTimeRepeat (Math|Float|Clamp(Float) (- (Variables|Default|GetTimeRepeat) (Utilities|Time|GetWorldDeltaSeconds)) 0.0 (Variables|Default|GetTimeRepeat)))
  (if (Variables|Default|Getwingame)
    (CallFunction|Win)
    (Variables|/Script/Engine.CharacterMovementComponent|SetMaxWalkSpeed _charactermovement (Variables|Default|GetDefaultSpeed))
    (Variables|/Script/Engine.CharacterMovementComponent|SetRotationRate _charactermovement (Variables|Default|GetRotation%20Rate))))

(event Custom|win
  (bind _returnvalue (Game|GetPlayerController 0))
  (Variables|Default|Set0-0 false)
  (Variables|Default|Set0-1 false)
  (Variables|Default|Set0-2 false)
  (Variables|Default|Set1-0 false)
  (Variables|Default|Set1-1 false)
  (Variables|Default|Set1-2 false)
  (Utilities|IsValid (stale OnComponentBeginOverlap(Box) _returnvalue)
    (:Is%20Valid
      (Widget|RemovefromParent (stale OnComponentBeginOverlap(Box) _returnvalue))
      (Input|SetInputModeGameOnly _returnvalue)
      (Input|EnableInput _returnvalue)
      (Development|PrintString "burada ui a return donecek")
      (Default|IncreaseResource (Variables|/Game/TopDown/Blueprints/BP_TopDownCharacter.BP_TopDownCharacter_C|GetInventoryComponent (Variables|Default|GetAs%20BP%20Top%20Down%20Character)) (Variables|Default|GetPrizeResource))
      (Utilities|IsValid _returnvalue
        (:Is%20Valid
          (Actor|DestroyActor)
          (CallFunction|Tekrarla))))))

(event Custom|lose)

(event EventBeginPlay
  (Variables|Default|Set0-0 false)
  (Variables|Default|Set0-1 false)
  (Variables|Default|Set0-2 false)
  (Variables|Default|Set1-0 false)
  (Variables|Default|Set1-1 false)
  (Variables|Default|Set1-2 false)
  (bind _asbp_top_down_character (Utilities|Casting|CastToBP_TopDownCharacter (Game|GetPlayerCharacter 0)))
  (bind _output_get (Variables|Default|SetAs%20BP%20Top%20Down%20Character _asbp_top_down_character))
  (Variables|Default|SetDefaultSpeed (Class|MovementComponent|GetMaxSpeed (Variables|/Script/Engine.Character|GetCharacterMovement _output_get)))
  (Variables|Default|SetRotation%20Rate (Variables|/Script/Engine.CharacterMovementComponent|GetRotationRate (Variables|/Script/Engine.Character|GetCharacterMovement _output_get))))

(event Collision|EventActorBeginOverlap
  (params (OtherActor :type Actor%20Object%20Reference)))

(event EventTick
  (params (DeltaSeconds :type Float%20%28single-precision%29))
  (CallFunction|Timer))

(fn ConstructionScript)

(fn F1-0
  (Variables|Default|Set1-0 true))

(fn F1-1
  (Variables|Default|Set1-1 true))

(fn F1-2
  (Variables|Default|Set1-2 true))

(fn Tekrarla
  (return))

(fn F0-0
  (Variables|Default|Set0-0 true))

(fn F0-1
  (Variables|Default|Set0-1 true))

(fn F0-2
  (Variables|Default|Set0-2 true))