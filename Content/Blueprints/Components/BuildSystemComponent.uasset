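; Build-mode component for BP_TopDownCharacter, toggled with X, that previews and places a building.
; While active, Tick traces from the camera and moves a preview mesh component, created once per session, to the hit point.
; Enter reads overlap and cost from an existing SpawnObject instance found by GetActorOfClass, deducts resources through InventoryComponent, then spawns SpawnObject or turns the preview red if IsCanBuild is false.
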(event Custom|PreviewLoop
  (bind _camera (Variables|Default|GetCamera))
  (bind _returnvalue (Transformation|GetWorldTransform _camera))
  (bind (_outhit _returnvalue_2) (Collision|LineTraceByChannel (.location _returnvalue) (+ (.location _returnvalue) (* (Math|Vector|GetForwardVector (.rotation _returnvalue)) 3e+03) "0.000000,200.000000,200.000000") "TraceTypeQuery1" false 0 "ForOneFrame"))
  (if _returnvalue_2
    (Utilities|FlowControl|Sequence
      (:then_0
        (Utilities|FlowControl|DoOnce false
          (:Completed
            (bind _returnvalue_3 (Game|AddComponentbyClass (Variables|Default|GetAs%20BP%20Top%20Down%20Character) "/Script/Engine.StaticMeshComponent" false (Variables|Default|GetBuild%20Preview%20Transform)))
            (Variables|Default|SetPreview%20Mesh _returnvalue_3)
            (Rendering|Material|SetMaterial (Variables|Default|GetPreview%20Mesh) 0 "/Game/Blueprints/M_Building_Preview.M_Building_Preview"))))
      (:then_1
        (bind _output_get (Variables|Default|SetBuild%20Preview%20Transform (Math|Transform|MakeTransform (.Location (Collision|BreakHitResult _outhit)) "0, 0, 0" "1.000000,1.000000,1.000000")))
        (Transformation|SetWorldTransform (Variables|Default|GetPreview%20Mesh) _output_get false false)))))

(event Custom|ResetBuildMode
  (Utilities|FlowControl|DoOnce false) ; enters at Reset
)

(event EventBeginPlay
  (bind _asbp_top_down_character (Utilities|Casting|CastToBP_TopDownCharacter (Components|GetOwner)))
  (Variables|Default|SetAs%20BP%20Top%20Down%20Character _asbp_top_down_character)
  (Variables|Default|SetCamera (Variables|/Game/TopDown/Blueprints/BP_TopDownCharacter.BP_TopDownCharacter_C|GetCamera _asbp_top_down_character)))

(event EventTick
  (params (DeltaSeconds :type Float%20%28single-precision%29))
  (if (Variables|Default|GetBuildMode)
    (CallFunction|PreviewLoop)))

(event Input|KeyboardEvents|X
  (params (Key :type Key%20Structure :default "None"))
  (:Pressed
    (Utilities|FlowControl|FlipFlop
      (:A
        (Variables|Default|SetBuildMode true))
      (:B
        (Variables|Default|SetBuildMode false)
        (Components|StaticMesh|SetStaticMesh (Variables|Default|GetPreview%20Mesh) 0)
        (Variables|Default|SetPreview%20Mesh 0)
        (CallFunction|ResetBuildMode)))))

(event Input|KeyboardEvents|Enter
  (params (Key :type Key%20Structure :default "None"))
  (bind _as_bp_top_down_character (Variables|Default|GetAs%20BP%20Top%20Down%20Character))
  (bind _inventorycomponent (Variables|/Game/TopDown/Blueprints/BP_TopDownCharacter.BP_TopDownCharacter_C|GetInventoryComponent _as_bp_top_down_character))
  (:Pressed
    (if (Variables|Default|GetBuildMode)
      (bind _returnvalue (Actor|GetActorOfClass (Variables|Default|GetSpawnObject)))
      (bind _asbp_building (Utilities|Casting|CastToBP_Building _returnvalue))
      (if (not (Variables|/Game/Blueprints/BP_Building.BP_Building_C|GetIsInteractEachOther _asbp_building))
        (Default|DecreaseResource _inventorycomponent (Variables|/Game/Blueprints/BP_Building.BP_Building_C|GetDesiredResource _asbp_building))
        (if (Variables|/Game/Blueprints/Components/InventoryComponent.InventoryComponent_C|GetIsCanBuild _inventorycomponent)
          (Game|SpawnActorfromClass (Variables|Default|GetSpawnObject) (Variables|Default|GetBuild%20Preview%20Transform) "AlwaysSpawn" 0 0)
          (else
            (Rendering|Material|SetMaterial (Variables|Default|GetPreview%20Mesh) 0 "/Game/Blueprints/M_Red_Building_Preview.M_Red_Building_Preview")))))))