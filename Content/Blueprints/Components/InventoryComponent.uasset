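; Inventory component that stores a struct of crafting resources (iron, copper, glass, battery, seed) and gates building on their availability.
; IncreaseResource adds a prize struct to MyInventory member by member.
; DecreaseResource checks each resource in turn, subtracting the whole cost and setting IsCanBuild true only if all suffice.
; Otherwise it zeroes the first insufficient resource, prints Turkish shortage messages and sets IsCanBuild false.
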(event EventBeginPlay)

(event EventTick
  (params (DeltaSeconds :type Float%20%28single-precision%29)))

(fn IncreaseResource
  (params (PrizeResources :type Inventory%20Structure))
  (Variables|Default|SetMyInventory (Utilities|Struct|MakeInventory (+ (.iron (Variables|Default|GetMyInventory)) (.iron PrizeResources)) (+ (.copper (Variables|Default|GetMyInventory)) (.copper PrizeResources)) (+ (.glass (Variables|Default|GetMyInventory)) (.glass PrizeResources)) (+ (.battery (Variables|Default|GetMyInventory)) (.battery PrizeResources)) (+ (.seed (Variables|Default|GetMyInventory)) (.seed PrizeResources)))))

(fn DecreaseResource
  (params (DesiredResources :type Inventory%20Structure))
  (if (>= (- (.iron (Variables|Default|GetMyInventory)) (.iron DesiredResources)) 0)
    (if (>= (- (.copper (Variables|Default|GetMyInventory)) (.copper DesiredResources)) 0)
      (if (>= (- (.glass (Variables|Default|GetMyInventory)) (.glass DesiredResources)) 0)
        (if (>= (- (.battery (Variables|Default|GetMyInventory)) (.battery DesiredResources)) 0)
          (if (>= (- (.seed (Variables|Default|GetMyInventory)) (.seed DesiredResources)) 0)
            (Variables|Default|SetMyInventory (Utilities|Struct|MakeInventory (- (.iron (Variables|Default|GetMyInventory)) (.iron DesiredResources)) (- (.copper (Variables|Default|GetMyInventory)) (.copper DesiredResources)) (- (.glass (Variables|Default|GetMyInventory)) (.glass DesiredResources)) (- (.battery (Variables|Default|GetMyInventory)) (.battery DesiredResources)) (- (.seed (Variables|Default|GetMyInventory)) (.seed DesiredResources))))
            (Variables|Default|SetIsCanBuild true)
            (else
              (Utilities|Struct|SetmembersinInventory (Variables|Default|GetMyInventory))
              (Development|PrintString "Tohum kalmadi")
              (Development|PrintString "insa edilemez")
              (Variables|Default|SetIsCanBuild false)))
          (else
            (Utilities|Struct|SetmembersinInventory (Variables|Default|GetMyInventory))
            (Development|PrintString "Pil kalmadi")
            (Development|PrintString "insa edilemez")
            (Variables|Default|SetIsCanBuild false)))
        (else
          (Utilities|Struct|SetmembersinInventory (Variables|Default|GetMyInventory))
          (Development|PrintString "Cam kalmadi")
          (Development|PrintString "insa edilemez")
          (Variables|Default|SetIsCanBuild false)))
      (else
        (Utilities|Struct|SetmembersinInventory (Variables|Default|GetMyInventory))
        (Development|PrintString "Bakir kalmadi")
        (Development|PrintString "insa edilemez")
        (Variables|Default|SetIsCanBuild false)))
    (else
      (Utilities|Struct|SetmembersinInventory (Variables|Default|GetMyInventory))
      (Development|PrintString "Demir kalmadı")
      (Development|PrintString "insa edilemez")
      (Variables|Default|SetIsCanBuild false))))