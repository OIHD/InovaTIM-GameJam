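; BP_PuzzleMiniGame is a trigger actor that starts a jigsaw puzzle minigame on box overlap.
; BeginPlay caches the top-down character, its movement speed, rotation rate and player controller.
; Overlap freezes that character, plays an interact montage, then after a short delay opens JigsawWidget with UI-only input.
; FinishGame destroys the actor; the saved movement values are not restored here.
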(event OnComponentBeginOverlap(Box)
  (params (OverlappedComponent :type Primitive%20Component%20Object%20Reference) (OtherActor :type Actor%20Object%20Reference) (OtherComp :type Primitive%20Component%20Object%20Reference) (OtherBodyIndex :type Integer) (bFromSweep :type Boolean) (SweepResult :type Hit%20Result%20Structure%20%28by%20ref%29))
  (bind _as_bp_top_down_character (Variables|Default|GetAs%20BP%20Top%20Down%20Character))
  (bind _charactermovement (Variables|/Script/Engine.Character|GetCharacterMovement _as_bp_top_down_character))
  (Variables|/Script/Engine.CharacterMovementComponent|SetMaxWalkSpeed _charactermovement 0.0)
  (Variables|/Script/Engine.CharacterMovementComponent|SetRotationRate _charactermovement "0, 0, 0")
  (Animation|Montage|PlayMontage (Variables|/Script/Engine.Character|GetMesh _as_bp_top_down_character) "/Game/Models/Character_Main/mc-robot_Anim_Interact_Montage.mc-robot_Anim_Interact_Montage"
    (:then
      (Utilities|FlowControl|Delay 0.5)
      (bind _returnvalue (UserInterface|CreateWidget "/Game/Jigsaw/JigsawWidget.JigsawWidget_C"))
      (UserInterface|Viewport|AddtoViewport _returnvalue 0)
      (Input|SetInputModeUIOnly (Variables|Default|GetAs%20Player%20Controller) _returnvalue "DoNotLock"))))

(event EventBeginPlay
  (bind _asbp_top_down_character (Utilities|Casting|CastToBP_TopDownCharacter (Game|GetPlayerCharacter 0)))
  (bind _output_get (Variables|Default|SetAs%20BP%20Top%20Down%20Character _asbp_top_down_character))
  (Variables|Default|SetDefaultSpeed (Class|MovementComponent|GetMaxSpeed (Variables|/Script/Engine.Character|GetCharacterMovement _output_get)))
  (Variables|Default|SetRotation%20Rate (Variables|/Script/Engine.CharacterMovementComponent|GetRotationRate (Variables|/Script/Engine.Character|GetCharacterMovement _output_get)))
  (bind _asplayer_controller (Utilities|Casting|CastToPlayerController (Pawn|GetController _asbp_top_down_character)))
  (Variables|Default|SetAs%20Player%20Controller _asplayer_controller))

(event EventTick
  (params (DeltaSeconds :type Float%20%28single-precision%29)))

(fn ConstructionScript)

(fn FinishGame
  (Actor|DestroyActor))