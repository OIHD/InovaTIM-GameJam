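; BP_EnemyAi is an enemy that chases a BP_Shield actor and takes damage from touching it.
; BeginPlay caches the shield reference, and Tick reissues AI MoveTo toward it every frame.
; Mesh overlap with the shield starts a looping timer that drains Health each second, until a Niagara shockwave spawns and the enemy is destroyed.
; The pawn-sensing player-follow logic is unwired.
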(event OnSeePawn(PawnSensing)
  (params (Pawn :type Pawn%20Object%20Reference)))

(event OnComponentBeginOverlap(Mesh)
  (params (OverlappedComponent :type Primitive%20Component%20Object%20Reference) (OtherActor :type Actor%20Object%20Reference) (OtherComp :type Primitive%20Component%20Object%20Reference) (OtherBodyIndex :type Integer) (bFromSweep :type Boolean) (SweepResult :type Hit%20Result%20Structure%20%28by%20ref%29))
  (Utilities|Casting|CastToBP_Shield OtherActor)
  (Utilities|Time|SetTimerbyEvent (delegate Custom|TakeDamage) 1.0 true))

(event Custom|FollowPlayer)

(event Custom|TakeDamage
  (Variables|Default|SetHealth (- (Variables|Default|GetHealth) 15.0))
  (if (<= (- (Variables|Default|GetHealth) 15.0) 0.0)
    (Niagara|SpawnSystematLocation "/Game/shieldEffect/NS_Shockwave.NS_Shockwave" (Transformation|GetActorLocation) "0.000000, 0,0.000000" "5.000000,5.000000,5.000000")
    (Utilities|FlowControl|Delay 0.2)
    (Actor|DestroyActor)
    (else
      (Development|PrintString (Utilities|String|ToString(Float) (- (Variables|Default|GetHealth) 15.0))))))

(event EventBeginPlay
  (bind _outactors (Actor|GetAllActorsOfClass 0))
  (for _array_element _outactors
    (bind _asbp_shield (Utilities|Casting|CastToBP_Shield _array_element))
    (Variables|Default|SetAs%20BP%20Shield _asbp_shield)))

(event Collision|EventActorBeginOverlap
  (params (OtherActor :type Actor%20Object%20Reference)))

(event EventTick
  (params (DeltaSeconds :type Float%20%28single-precision%29))
  (AI|AIMoveTo self "0, 0, 0" (Variables|Default|GetAs%20BP%20Shield) 5.0 false
    (:OnSuccess
      (Development|PrintString "1"))
    (:OnFail
      (Development|PrintString "2"))))

(fn ConstructionScript)